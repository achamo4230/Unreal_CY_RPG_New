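; BP_帽女 is the player character (hat girl), who fights zombies and picks up keys.
; Input drives camera-relative movement, sprint and a weapon toggle that reattaches it between hand and back mid-montage.
; Light and heavy attacks alternate two montages using DoOnce gates and delayed combo resets.
; The weapon's overlap box damages BP_殭屍, with toggle functions for its overlaps and movement; 帽女受傷 handles damage and death, and BeginPlay adds the UI.
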(event `InputAxis|Turn` :overrideparent false
  (params (AxisValue :type "Float (single-precision)"))
  ;[1 1 1] 滑鼠操作
  (`self.AddControllerYawInput` AxisValue))

(event `InputAxis|MoveForward` :overrideparent false
  (params (AxisValue :type "Float (single-precision)"))
  ;[1 1 1] 移動
  (if (`self.是否移動`)
    (`self.AddMovementInput` (`KismetMathLibrary.GetForwardVector` (`KismetMathLibrary.MakeRotator` 0.0 0.0 (.yaw (`self.GetControlRotation`)))) AxisValue)))

(event `InputAxis|LookUp` :overrideparent false
  (params (AxisValue :type "Float (single-precision)"))
  ;[1 1 1] 滑鼠操作
  (`self.AddControllerPitchInput` AxisValue))

(event `InputAxis|MoveRight` :overrideparent false
  (params (AxisValue :type "Float (single-precision)"))
  ;[1 1 1] 移動
  (if (`self.是否移動`)
    (`self.AddMovementInput` (`KismetMathLibrary.GetRightVector` (`KismetMathLibrary.MakeRotator` 0.0 0.0 (.yaw (`self.GetControlRotation`)))) AxisValue)))

(event `InputAction|衝刺`
  (params (Key :type "Key Structure"))
  (bind _charactermovement (`self.CharacterMovement`))
  ;[1 1 1] 衝刺
  (:`Pressed`
    (set `CharacterMovementComponent.MaxWalkSpeed` 800.0 _charactermovement))
  (:`Released`
    (set `CharacterMovementComponent.MaxWalkSpeed` 400.0 _charactermovement)))

(event `InputAction|武器切換`
  (params (Key :type "Key Structure"))
  (bind `_武器` (`self.武器`))
  ;[1 1 1] 取出/收回武器
  (:`Pressed`
    (set `self.切換武器` (not (`self.切換武器`)))
    (`|PlayMontage` (`self.Mesh`) "/Game/動畫/切換武器_M.切換武器_M" 1.5 ; 播放剪輯動畫
      (:`then`
        (if (`self.切換武器`)
          (`KismetSystemLibrary.Delay` 0.4) ; 延遲
          (`SceneComponent.K2_AttachToComponent` `_武器` (`self.右手位置`) "None" "KeepRelative" "KeepRelative" "KeepRelative" true) ; 拿武器：武器放在右手
          (else
            (`KismetSystemLibrary.Delay` 0.4) ; 延遲
            (`SceneComponent.K2_AttachToComponent` `_武器` (`self.右背位置`) "None" "KeepRelative" "KeepRelative" "KeepRelative" true) ; 拿武器：武器放回背後
          ))
        (`KismetSystemLibrary.MoveComponentTo` `_武器`) ; 移動元件到指定位置
      ))))

(event `InputAction|輕攻擊`
  (params (Key :type "Key Structure"))
  ;[1 1 1] 輕攻擊
  (:`Pressed`
    (`/Engine/EditorBlueprintResources/StandardMacros.DoOnce` false :!label _label
      (:`Completed`
        (if (`self.切換武器`)
          (`|PlayMontage` (`self.Mesh`) (select `int` (mod (`self.第一段攻擊`) 2) :`0` "/Game/動畫/輕攻擊第一段_Montage.輕攻擊第一段_Montage" :`1` "/Game/動畫/輕攻擊第二段_Montage.輕攻擊第二段_Montage" :!type "AnimMontage Object Reference") 1.1
            (:`then`
              (bind _result (`/Engine/EditorBlueprintResources/StandardMacros.IncrementInt` (`self.第一段攻擊`))
                (:`  `
                  (`KismetSystemLibrary.PrintString` (`KismetStringLibrary.Conv_IntToString` _result)) ; 輸入訊息：測試用
                  (`KismetSystemLibrary.Delay` 0.6) ; 延遲
                  (`|ExecutionSequence`
                    (:`then_0`
                      (goto _label :!via `Reset`))
                    (:`then_1`
                      (`KismetSystemLibrary.Delay` 1.1)
                      (set `self.第一段攻擊` 0)))))))
          (else
            (goto _label :!via `Reset`)))))))

(event `InputAction|重攻擊`
  (params (Key :type "Key Structure"))
  ;[1 1 1] 重攻擊
  (:`Pressed`
    (`/Engine/EditorBlueprintResources/StandardMacros.DoOnce` false :!label _label_2
      (:`Completed`
        (if (`self.切換武器`)
          (`|PlayMontage` (`self.Mesh`) (select `int` (mod (`self.第一段重攻擊`) 2) :`0` "/Game/動畫/重攻擊第一段_Montage.重攻擊第一段_Montage" :`1` "/Game/動畫/重攻擊第二段__2__Montage.重攻擊第二段__2__Montage" :!type "AnimMontage Object Reference")
            (:`then`
              (bind _result (`/Engine/EditorBlueprintResources/StandardMacros.IncrementInt` (`self.第一段重攻擊`))
                (:`  `
                  (`KismetSystemLibrary.PrintString` (`KismetStringLibrary.Conv_IntToString` _result)) ; 輸入訊息：測試用
                  (`KismetSystemLibrary.Delay` 1.7)
                  (`|ExecutionSequence`
                    (:`then_0`
                      (goto _label_2 :!via `Reset`))
                    (:`then_1`
                      (`KismetSystemLibrary.Delay` 3.0)
                      (set `self.第一段重攻擊` 0)))))))
          (else
            (goto _label_2 :!via `Reset`)))))))

(event `self.ReceiveBeginPlay`
  ;[1 1 1] 介面
  (bind _returnvalue (`|CreateWidget` "/Game/BP/BW_介面.BW_介面_C" (`GameplayStatics.GetPlayerController` 0)))
  (`UserWidget.AddToViewport` _returnvalue 0))

(event `self.武器碰撞區域.OnComponentBeginOverlap`
  (params (OverlappedComponent :type "PrimitiveComponent Object Reference") (OtherActor :type "Actor Object Reference") (OtherComp :type "PrimitiveComponent Object Reference") (OtherBodyIndex :type Integer) (bFromSweep :type Boolean) (SweepResult :type "HitResult Structure (by ref)"))
  (bind `_asbp_殭屍` (cast `/Game/BP/BP_殭屍` OtherActor))
  (`/Game/BP/BP_殭屍.殭屍受傷` `_asbp_殭屍` 30.0))

(event `self.ReceiveTick`
  (params (DeltaSeconds :type "Float (single-precision)"))
  (if (<= (`self.血量`) 0.0)
    (set `self.是否死亡` true)
    (`/Engine/EditorBlueprintResources/StandardMacros.DoOnce` false)))

(event `self.CapsuleComponent.OnComponentBeginOverlap`
  (params (OverlappedComponent :type "PrimitiveComponent Object Reference") (OtherActor :type "Actor Object Reference") (OtherComp :type "PrimitiveComponent Object Reference") (OtherBodyIndex :type Integer) (bFromSweep :type Boolean) (SweepResult :type "HitResult Structure (by ref)"))
  (bind `_聲音` (`self.聲音`))
  ;[1 1 1] 角色碰撞物件
  (bind `_asbp_鑰匙` (cast `/Game/BP/BP_鑰匙` OtherActor))
  (`AudioComponent.SetSound` `_聲音` "/Game/聲音/檢取物品.檢取物品")
  (`AudioComponent.Play` `_聲音` 0.0)
  (`self.K2_DestroyActor` `_asbp_鑰匙`)
  (`/Engine/EditorBlueprintResources/StandardMacros.IncrementInt` (`self.鑰匙數量`)))

(fn `UserConstructionScript`)

(fn `切換武器碰撞區域`
  (params (`是否顯示武器的攻擊範圍` :type Boolean))
  (set `PrimitiveComponent.bGenerateOverlapEvents` `是否顯示武器的攻擊範圍` (`self.武器碰撞區域`)))

(fn `切換移動`
  (params (`是否移動` :type Boolean))
  (set `self.是否移動` `是否移動`))

(fn `帽女受傷`
  (params (`傷害值` :type "Float (double-precision)"))
  (if (not (`self.是否死亡`))
    (set `self.血量` (- (`self.血量`) `傷害值`))
    (`self.PlayAnimMontage` self "/Game/動畫/角色受傷_Montage.角色受傷_Montage" 1.0 "None")
    (if (<= (`self.血量`) 0.0)
      (`self.PlayAnimMontage` self "/Game/動畫/角色死亡_Montage.角色死亡_Montage" 1.0 "None"))))