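; Zombie enemy Blueprint that wanders, chases the player character BP_帽女, attacks and dies.
; It roams to random reachable points until PawnSensing spots the player, then moves in and plays a DoOnce-gated attack montage before returning to wandering.
; A right-hand overlap volume, switchable by function, damages the player on contact.
; 殭屍受傷 subtracts health and plays hit or death montages, while Tick destroys the actor shortly after health runs out.
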(event `self.ReceiveBeginPlay`
  ;[1 1 1] AI隨機移動
  (`/Engine/EditorBlueprintResources/StandardMacros.IsValid` (`self.帽女物件`) :!label _label ; 如果玩家不存在時才隨機走動
    (:`Is Not Valid`
      (`|AIMoveTo` self (`NavigationSystemV1.K2_GetRandomReachablePointInRadius` (`SceneComponent.K2_GetComponentLocation` (`self.Mesh`)) 1000.0 null null) null ; AI前往指定位置
        (:`OnSuccess`
          _)
        (:`OnFail`
          _))
      (`KismetSystemLibrary.Delay` (`KismetMathLibrary.RandomFloatInRange` 0.5 2.0))
      (if (not (`self.攻擊玩家`)) :!label _label_2
        (goto _label)))))

(event `self.PawnSensing.OnSeePawn`
  (params (Pawn :type "Pawn Object Reference"))
  ;[1 1 1] AI追蹤角色
  (if (not (`self.攻擊玩家`))
    (bind `_asbp_帽女` (cast `/Game/BP/BP_帽女` Pawn))
    (bind _output_get (set `self.帽女物件` `_asbp_帽女`))
    (`|AIMoveTo` self (0.0 0.0 0.0) _output_get
      (:`OnSuccess`
        (`/Engine/EditorBlueprintResources/StandardMacros.DoOnce` false :!label _label_3
          (:`Completed`
            (`|PlayMontage` (`self.Mesh`) "/Game/敵人動畫/殭屍攻擊_Montage.殭屍攻擊_Montage"
              (:`then`
                (set `self.攻擊玩家` true)
                (set `self.帽女物件` null))
              (:`OnCompleted`
                (set `self.攻擊玩家` false)
                (`KismetSystemLibrary.Delay` 0.3)
                (`|ExecutionSequence`
                  (:`then_0`
                    (goto _label_3 :!via `Reset`))
                  (:`then_1`
                    (goto _label_2)))))))))))

(event `self.ReceiveTick`
  (params (DeltaSeconds :type "Float (single-precision)"))
  ;[1 1 1] AI血量<=0時死亡並消失
  (if (<= (`self.血量`) 0.0)
    (set `self.是否死亡` true)
    (`/Engine/EditorBlueprintResources/StandardMacros.DoOnce` false
      (:`Completed`
        (`KismetSystemLibrary.Delay` 2.0)
        (`self.K2_DestroyActor` self) ; 刪除
      ))))

(event `self.殭屍右手攻擊範圍.OnComponentBeginOverlap`
  (params (OverlappedComponent :type "PrimitiveComponent Object Reference") (OtherActor :type "Actor Object Reference") (OtherComp :type "PrimitiveComponent Object Reference") (OtherBodyIndex :type Integer) (bFromSweep :type Boolean) (SweepResult :type "HitResult Structure (by ref)"))
  (bind `_asbp_帽女` (cast `/Game/BP/BP_帽女` OtherActor))
  (`/Game/BP/BP_帽女.帽女受傷` `_asbp_帽女` 0.1))

(fn `UserConstructionScript`)

(fn `切換殭屍右手攻擊的區域`
  (params (`是否顯示殭屍右手攻擊的區域` :type Boolean))
  (set `PrimitiveComponent.bGenerateOverlapEvents` `是否顯示殭屍右手攻擊的區域` (`self.殭屍右手攻擊範圍`)))

(fn `殭屍受傷`
  (params (`傷害值` :type "Float (double-precision)"))
  (if (not (`self.是否死亡`))
    (set `self.血量` (- (`self.血量`) `傷害值`)) ; 設定血量
    (`self.PlayAnimMontage` self "/Game/敵人動畫/殭屍受傷_Montage.殭屍受傷_Montage" 1.0 "None")
    (if (<= (`self.血量`) 0.0)
      (`self.PlayAnimMontage` self "/Game/敵人動畫/殭屍死亡_Montage.殭屍死亡_Montage" 1.0 "None"))))